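; Wall-eye actor whose three eye components (Oeil, Oeil1, Oeil2) constantly stare at the player.
; Every Tick calls Lookatplayer, which casts player 0 to BP_FirstPersonCharacter and aims each eye separately at the FirstPersonCamera position with FindLookAtRotation.
; Fixed roll and yaw offsets are added to each look-at rotation before it is applied in world space.
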(event `self.ReceiveTick`
  (params (DeltaSeconds :type "Float (single-precision)"))
  (`self.lookatplayer`))

(fn `lookatplayer`
  (bind _oeil2 (`self.Oeil2`))
  (bind _oeil (`self.Oeil`))
  (bind _oeil1 (`self.Oeil1`))
  (bind _asbp_first_person_character (cast `/Game/FirstPerson/Blueprints/BP_FirstPersonCharacter` (`GameplayStatics.GetPlayerCharacter` 0)))
  (bind _returnvalue_location (`KismetMathLibrary.BreakTransform` (`SceneComponent.K2_GetComponentToWorld` (`/Game/FirstPerson/Blueprints/BP_FirstPersonCharacter.FirstPersonCamera` _asbp_first_person_character))))
  (bind (_returnvalue_roll _returnvalue_pitch _returnvalue_yaw) (`KismetMathLibrary.BreakRotator` (`KismetMathLibrary.FindLookAtRotation` (`SceneComponent.K2_GetComponentLocation` _oeil) _returnvalue_location)))
  (`SceneComponent.K2_SetWorldRotation` _oeil (`KismetMathLibrary.MakeRotator` (+ _returnvalue_roll 90.0) _returnvalue_pitch (+ _returnvalue_yaw -90.0)) false false)
  (bind _returnvalue_location_2 (`KismetMathLibrary.BreakTransform` (`SceneComponent.K2_GetComponentToWorld` (`/Game/FirstPerson/Blueprints/BP_FirstPersonCharacter.FirstPersonCamera` _asbp_first_person_character))))
  (bind (_returnvalue_roll_2 _returnvalue_pitch_2 _returnvalue_yaw_2) (`KismetMathLibrary.BreakRotator` (`KismetMathLibrary.FindLookAtRotation` (`SceneComponent.K2_GetComponentLocation` _oeil1) _returnvalue_location_2)))
  (`SceneComponent.K2_SetWorldRotation` _oeil1 (`KismetMathLibrary.MakeRotator` (+ _returnvalue_roll_2 90.0) _returnvalue_pitch_2 (+ _returnvalue_yaw_2 -90.0)) false false)
  (bind _returnvalue_location_3 (`KismetMathLibrary.BreakTransform` (`SceneComponent.K2_GetComponentToWorld` (`/Game/FirstPerson/Blueprints/BP_FirstPersonCharacter.FirstPersonCamera` _asbp_first_person_character))))
  (bind (_returnvalue_roll_3 _returnvalue_pitch_3 _returnvalue_yaw_3) (`KismetMathLibrary.BreakRotator` (`KismetMathLibrary.FindLookAtRotation` (`SceneComponent.K2_GetComponentLocation` _oeil2) _returnvalue_location_3)))
  (`SceneComponent.K2_SetWorldRotation` _oeil2 (`KismetMathLibrary.MakeRotator` (+ _returnvalue_roll_3 90.0) _returnvalue_pitch_3 (+ _returnvalue_yaw_3 -90.0)) false false))

(fn `UserConstructionScript`)