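; Quest manager actor that runs a random sequence of objectives until the player completes the required count and wins.
; On BeginPlay it shows the quest widget and gathers BP_Questable actors flagged as quests.
; RandQuest activates a random one, binds to its solved dispatcher and displays its objective.
; Each solve removes that quest and picks another, or fires the win dispatcher and shows the win screen.
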(event `self.ReceiveBeginPlay`
  (bind _returnvalue (`|CreateWidget` "/Game/ButcherProject/UI/WB_Quests.WB_Quests_C"))
  (bind _output_get (set `self.WB_Quest` _returnvalue))
  (`UserWidget.AddToViewport` _output_get 0)
  (bind _outactors (`GameplayStatics.GetAllActorsOfClass` "/Game/ButcherProject/Blueprints/BP_Questable.BP_Questable_C"))
  (for _array_element _outactors
    (bind (_dataquest_isactive _dataquest_isended _dataquest_questtype _dataquest_objectif _dataquest_id _dataquest_isquest) (break `/Game/ButcherProject/Blueprints/S_Quest` (`/Game/ButcherProject/Blueprints/BP_Questable.DataQuest` _array_element)))
    (if _dataquest_isquest
      (`KismetArrayLibrary.Array_Add` (`self.ListRefQuest`) _array_element)))
  (`self.RandQuest`))

(event `self.ReceiveTick`
  (params (DeltaSeconds :type "Float (single-precision)")))

(event `CE_BindManagerToCurrentQuest`
  (bind _currentquest (`self.CurrentQuest`))
  (bind (_dataquest_isactive _dataquest_isended _dataquest_questtype _dataquest_objectif _dataquest_id) (break `/Game/ButcherProject/Blueprints/S_Quest` (`/Game/ButcherProject/Blueprints/BP_Questable.DataQuest` _currentquest)))
  (add `/Game/ButcherProject/Blueprints/BP_Questable.ED_QuestSolved` _currentquest (delegate `CustomEvent`))
  (`KismetSystemLibrary.PrintString` (`KismetStringLibrary.Concat_StrStr` _dataquest_id ": binded")))

(event `CustomEvent`
  (`KismetSystemLibrary.PrintString` "QuestSolved")
  (`KismetArrayLibrary.Array_RemoveItem` (`self.ListRefQuest`) (`self.CurrentQuest`))
  (`/Engine/EditorBlueprintResources/StandardMacros.IncrementInt` (`self.NQuestDone`)
    (:`  `
      (if (< (`self.NQuestDone`) (`self.NQuestToDo`))
        (`self.RandQuest`)
        (else
          (set `self.CurrentQuest` null)
          (`KismetSystemLibrary.PrintString` "YOUWIN")
          (`self.ED_WIN`)
          (bind _returnvalue (`|CreateWidget` "/Game/ButcherProject/UI/WB_Win.WB_Win_C" (`GameplayStatics.GetPlayerController` 0)))
          (`UserWidget.AddToViewport` _returnvalue 0))))))

(fn `RandQuest`
  (bind _currentquest (`self.CurrentQuest`))
  (bind (_dataquest_isactive _dataquest_isended _dataquest_questtype _dataquest_objectif _dataquest_id) (break `/Game/ButcherProject/Blueprints/S_Quest` (`/Game/ButcherProject/Blueprints/BP_Questable.DataQuest` _currentquest)))
  (bind _output_get (set `self.CurrentQuest` (`KismetArrayLibrary.Array_Random` (`self.ListRefQuest`))))
  (`/Game/ButcherProject/Blueprints/BP_Questable.ActivateQuest` _output_get)
  (`KismetSystemLibrary.PrintString` (`KismetStringLibrary.Concat_StrStr` (`KismetSystemLibrary.GetObjectName` _currentquest) _dataquest_id))
  (`self.CE_BindManagerToCurrentQuest`)
  (`/Game/ButcherProject/UI/WB_Quests.SetTextQuest` (`self.WB_Quest`) _dataquest_objectif))

(fn `UserConstructionScript`)