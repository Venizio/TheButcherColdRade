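; AC_QuestPickUp is an actor component that manages the quest state of the BP_Questable actor that owns it.
; On BeginPlay it caches that owner.
; ActiveQuest flags the owner's DataQuest as active and broadcasts QuestActivated with the objective.
; SolveQuest marks it ended, fires QuestSolved on the component and EDQuestSolved on the owner, then hides the owner's Cube and its children.
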(event `self.ReceiveBeginPlay`
  (bind _asbp_questable (cast `/Game/ButcherProject/Blueprints/BP_Questable` (`self.GetOwner`)))
  (set `self.Owner_PickUp` _asbp_questable))

(fn `ActiveQuest`
  (bind _owner_pickup (`self.Owner_PickUp`))
  (bind (_dataquest_isactive _dataquest_isended _dataquest_questtype _dataquest_objectif _dataquest_id _dataquest_isquest) (break `/Game/ButcherProject/Blueprints/S_Quest` (`/Game/ButcherProject/Blueprints/BP_Questable.DataQuest` _owner_pickup)))
  (set `/Game/ButcherProject/Blueprints/BP_Questable.DataQuest` (make `/Game/ButcherProject/Blueprints/S_Quest` true _dataquest_isended _dataquest_questtype _dataquest_objectif _dataquest_id _dataquest_isquest) _owner_pickup)
  (`self.QuestActivated` _dataquest_objectif))

(fn `SolveQuest`
  (bind _owner_pickup (`self.Owner_PickUp`))
  (bind (_dataquest_isactive _dataquest_isended _dataquest_questtype _dataquest_objectif _dataquest_id _dataquest_isquest) (break `/Game/ButcherProject/Blueprints/S_Quest` (`/Game/ButcherProject/Blueprints/BP_Questable.DataQuest` _owner_pickup)))
  (set `/Game/ButcherProject/Blueprints/BP_Questable.DataQuest` (make `/Game/ButcherProject/Blueprints/S_Quest` false true _dataquest_questtype _dataquest_objectif _dataquest_id _dataquest_isquest) _owner_pickup)
  (`self.QuestSolved`)
  (`/Game/ButcherProject/Blueprints/BP_Questable.ED_QuestSolved` _owner_pickup)
  (`SceneComponent.SetVisibility` (`/Game/ButcherProject/Blueprints/BP_Questable.Cube` (`self.Owner_PickUp`)) false true))