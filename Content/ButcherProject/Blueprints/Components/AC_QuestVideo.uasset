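; Quest component for a BP_Questable owner that tracks one quest's state and announces its changes.
; On BeginPlay it copies the owner's DataQuest struct into its own variable, stopping if the owner is another class.
; ActiveQuest sets the struct's first flag and fires QuestActivated with the objective.
; SolveQuest clears that flag, marks the quest ended and fires QuestSolved; neither function writes back to the owner.
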(event `self.ReceiveBeginPlay`
  (bind _asbp_questable (cast `/Game/ButcherProject/Blueprints/BP_Questable` (`self.GetOwner`)))
  (set `self.DataQuest` (`/Game/ButcherProject/Blueprints/BP_Questable.DataQuest` _asbp_questable)))

(fn `ActiveQuest`
  (bind (_dataquest_isactive _dataquest_isended _dataquest_questtype _dataquest_objectif _dataquest_id) (break `/Game/ButcherProject/Blueprints/S_Quest` (`self.DataQuest`)))
  (set `self.DataQuest` (make `/Game/ButcherProject/Blueprints/S_Quest` true _dataquest_isended _dataquest_questtype _dataquest_objectif _dataquest_id))
  (`self.QuestActivated` _dataquest_objectif))

(fn `SolveQuest`
  (bind (_dataquest_isactive _dataquest_isended _dataquest_questtype _dataquest_objectif _dataquest_id) (break `/Game/ButcherProject/Blueprints/S_Quest` (`self.DataQuest`)))
  (set `self.DataQuest` (make `/Game/ButcherProject/Blueprints/S_Quest` false true _dataquest_questtype _dataquest_objectif _dataquest_id))
  (`self.QuestSolved`))