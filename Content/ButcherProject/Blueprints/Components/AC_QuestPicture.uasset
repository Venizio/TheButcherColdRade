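; Actor component that manages the quest state of its owning BP_Questable in the game.
; On BeginPlay it casts and caches the owner as OwnerPicture.
; ActiveQuest and SolveQuest rewrite the two leading flags of the owner's DataQuest struct to active or solved, keeping its other fields.
; Activation broadcasts QuestActivated with the objective, while solving broadcasts QuestSolved and also fires the owner's EDQuestSolved dispatcher.
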(event `self.ReceiveBeginPlay`
  (bind _asbp_questable (cast `/Game/ButcherProject/Blueprints/BP_Questable` (`self.GetOwner`)))
  (set `self.Owner_Picture` _asbp_questable))

(fn `ActiveQuest`
  (bind _owner_picture (`self.Owner_Picture`))
  (bind (_dataquest_isactive _dataquest_isended _dataquest_questtype _dataquest_objectif _dataquest_id _dataquest_isquest) (break `/Game/ButcherProject/Blueprints/S_Quest` (`/Game/ButcherProject/Blueprints/BP_Questable.DataQuest` _owner_picture)))
  (set `/Game/ButcherProject/Blueprints/BP_Questable.DataQuest` (make `/Game/ButcherProject/Blueprints/S_Quest` true false _dataquest_questtype _dataquest_objectif _dataquest_id _dataquest_isquest) _owner_picture)
  (`self.QuestActivated` _dataquest_objectif))

(fn `SolveQuest`
  (bind _owner_picture (`self.Owner_Picture`))
  (bind (_dataquest_isactive _dataquest_isended _dataquest_questtype _dataquest_objectif _dataquest_id _dataquest_isquest) (break `/Game/ButcherProject/Blueprints/S_Quest` (`/Game/ButcherProject/Blueprints/BP_Questable.DataQuest` _owner_picture)))
  (set `/Game/ButcherProject/Blueprints/BP_Questable.DataQuest` (make `/Game/ButcherProject/Blueprints/S_Quest` false true _dataquest_questtype _dataquest_objectif _dataquest_id _dataquest_isquest) _owner_picture)
  (`KismetSystemLibrary.PrintString` "FiniFromComp")
  (`self.QuestSolved`)
  (`/Game/ButcherProject/Blueprints/BP_Questable.ED_QuestSolved` (`self.Owner_Picture`)))