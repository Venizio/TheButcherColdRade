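; AC_Camera is a component on BP_FirstPersonCharacter that lets the player's camera complete photo and video quests.
; It binds to the owner's visibility events to keep a list of visible questables, firing WasRemoved when an active video target leaves view.
; Pic and Video events filter that list by active state and quest type, then call SolveQuest on each target's picture or video quest component.
; Picture saving is an unfinished, unused stub.
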(event `self.ReceiveBeginPlay`
  (bind _asbp_first_person_character (cast `/Game/FirstPerson/Blueprints/BP_FirstPersonCharacter` (`self.GetOwner`))
    (:`then`
      (bind _output_get (set `self.Owner` _asbp_first_person_character))
      (add `/Game/FirstPerson/Blueprints/BP_FirstPersonCharacter.IsVisible` _output_get (delegate `CE_IsVisible`))
      (add `/Game/FirstPerson/Blueprints/BP_FirstPersonCharacter.IsNotVisible` _output_get (delegate `CE_IsNotVisible`))
      (set `self.CaptureComp` (`/Game/FirstPerson/Blueprints/BP_FirstPersonCharacter.SceneCaptureComponent2D` _asbp_first_person_character))
      (bind _returnvalue (`GameplayStatics.GetActorOfClass` "/Game/ButcherProject/Blueprints/BP_QuestsManager.BP_QuestsManager_C"))
      (set `self.WB Quest` (`/Game/ButcherProject/Blueprints/BP_QuestsManager.WB_Quest` _returnvalue)))
    (:`CastFailed`
      (`KismetSystemLibrary.PrintString` "error"))))

(event `CE_IsVisible`
  (params (Questable :type "/Game/ButcherProject/Blueprints/BP_Questable Object Reference"))
  (`KismetArrayLibrary.Array_Add` (`self.Quests`) Questable))

(event `CE_IsNotVisible`
  (params (Questable :type "/Game/ButcherProject/Blueprints/BP_Questable Object Reference"))
  (bind (_dataquest_isactive _dataquest_isended _dataquest_questtype) (break `/Game/ButcherProject/Blueprints/S_Quest` (`/Game/ButcherProject/Blueprints/BP_Questable.DataQuest` Questable)))
  (`KismetArrayLibrary.Array_RemoveItem` (`self.Quests`) Questable)
  (if (and _dataquest_isactive (`|EnumEquality` _dataquest_questtype "NewEnumerator1"))
    (`self.WasRemoved`)))

(event `Pic`
  ;[1 1 1] TakePicture
  (for _array_element (`self.Quests`)
    (bind (_dataquest_isactive _dataquest_isended _dataquest_questtype) (break `/Game/ButcherProject/Blueprints/S_Quest` (`/Game/ButcherProject/Blueprints/BP_Questable.DataQuest` _array_element)))
    (if (and _dataquest_isactive (`|EnumEquality` _dataquest_questtype "NewEnumerator0"))
      (`/Game/ButcherProject/Blueprints/Components/AC_QuestPicture.SolveQuest` (`Actor.GetComponentByClass` _array_element "/Game/ButcherProject/Blueprints/Components/AC_QuestPicture.AC_QuestPicture_C")))))

(event `Video`
  (params (Stop :type Boolean))
  ;[1 1 1] Video
  (for _array_element (`self.Quests`)
    (bind (_dataquest_isactive _dataquest_isended _dataquest_questtype) (break `/Game/ButcherProject/Blueprints/S_Quest` (`/Game/ButcherProject/Blueprints/BP_Questable.DataQuest` _array_element)))
    (if (and _dataquest_isactive (`|EnumEquality` _dataquest_questtype "NewEnumerator1"))
      (`KismetSystemLibrary.PrintString` "true")
      (`/Game/ButcherProject/Blueprints/Components/AC_QuestVideo.SolveQuest` (`Actor.GetComponentByClass` _array_element "/Game/ButcherProject/Blueprints/Components/AC_QuestVideo.AC_QuestVideo_C") self Stop)
      (else
        (`KismetSystemLibrary.PrintString` "false")))))

(fn `SavePicture`)