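; BP_Enemy is the butcher enemy character, which plays ambient sounds and kills the player on touch.
; Looping timers with randomized intervals, set at BeginPlay, play spatialized tool and growl sounds at its location.
; A capsule overlap with the tagged player, gated by a DoOnce, plays death sounds, destroys the character, then after a delay spawns and possesses a new one at Playerstart.
; UpdateWalkSpeed sets its max walk speed.
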(event `self.ReceiveBeginPlay`
  ;[1 1 1] ToolsSound
  (`KismetSystemLibrary.K2_SetTimerDelegate` (delegate `StartToolsSound`) (`KismetMathLibrary.RandomFloatInRange` 5.0 15.0) true)
  ;[1 1 1] GruntSound
  (`KismetSystemLibrary.K2_SetTimerDelegate` (delegate `StartGruntSound`) (`KismetMathLibrary.RandomFloatInRange` 6.0 20.0) true))

(event `StartToolsSound`
  ;[1 1 1] ToolsSound
  (`GameplayStatics.PlaySoundAtLocation` "/Game/ButcherProject/Sounds/Music/MS_ToolsSound.MS_ToolsSound" (`self.K2_GetActorLocation`) (struct) 1.0 1.0 0.0 (`self.Attenuation Settings`) null null null))

(event `StartGruntSound`
  ;[1 1 1] GruntSound
  (`GameplayStatics.PlaySoundAtLocation` "/Game/ButcherProject/Sounds/Music/MS_GrowlSound.MS_GrowlSound" (`self.K2_GetActorLocation`) (struct) 1.0 1.0 0.0 (`self.Attenuation Settings`) null null null))

(event `self.CapsuleComponent.OnComponentBeginOverlap`
  (params (OverlappedComponent :type "PrimitiveComponent Object Reference") (OtherActor :type "Actor Object Reference") (OtherComp :type "PrimitiveComponent Object Reference") (OtherBodyIndex :type Integer) (bFromSweep :type Boolean) (SweepResult :type "HitResult Structure (by ref)"))
  (bind _returnvalue (`self.K2_GetActorLocation`))
  ;[1 1 1] Death and respawn
  (bind _asbp_first_person_character (cast `/Game/FirstPerson/Blueprints/BP_FirstPersonCharacter` OtherActor))
  (if (`self.ActorHasTag` _asbp_first_person_character "Player")
    (`/Engine/EditorBlueprintResources/StandardMacros.DoOnce` false :!label _label
      (:`Completed`
        (`GameplayStatics.PlaySoundAtLocation` "/Game/ButcherProject/Sounds/SFX/Hit_Suspens.Hit_Suspens" _returnvalue (struct) 1.0 1.0 0.0 "/Game/ButcherProject/Sounds/SFX/SoundAttenuationEnemy.SoundAttenuationEnemy" null null null)
        (`GameplayStatics.PlaySoundAtLocation` "/Game/ButcherProject/Sounds/SFX/MS_DiyingSound.MS_DiyingSound" _returnvalue (struct) 1.0 1.0 0.0 "/Game/ButcherProject/Sounds/SFX/SoundAttenuationEnemy.SoundAttenuationEnemy" null null null)
        (`self.K2_DestroyActor` _asbp_first_person_character)
        (`KismetSystemLibrary.Delay` 4.0)
        (bind _returnvalue_2 (`|SpawnActorFromClass` "/Game/FirstPerson/Blueprints/BP_FirstPersonCharacter.BP_FirstPersonCharacter_C" (`self.GetTransform` (`self.Playerstart`)) "AdjustIfPossibleButAlwaysSpawn" "MultiplyWithRoot" null null))
        (`Controller.Possess` (`GameplayStatics.GetPlayerController` 0) _returnvalue_2)
        (goto _label :!via `Reset`)))))

(fn `UpdateWalkSpeed`
  (params (NewWalkSpeed :type "Float (double-precision)"))
  (set `CharacterMovementComponent.MaxWalkSpeed` NewWalkSpeed (`self.CharacterMovement`)))

(fn `UserConstructionScript`)